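; Level objective manager for the ball game, tracking a level through start, win and fail states under one objective mode.
; Timed mode unlocks the finish immediately and runs a one-second looping countdown that fails at zero; otherwise registered pickups unlock it at the required count.
; TryFinish completes only when unlocked, then ReturnMainMenu opens the hard-coded Level2_Testing after a delay.
; Failure reloads the current level, and feedback uses debug prints.
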(event `self.ReceiveBeginPlay`
  (set `self.CurrentState` "NewEnumerator0")
  (set `self.CollectedItems` 0)
  (set `self.FinishUnlocked` false)
  (`KismetSystemLibrary.PrintString` (`KismetStringLibrary.Conv_IntToString` (`self.RequiredItems`)) true true (struct :`G` 0.66 :`B` 1.0 :`A` 1.0) 5.0))

(event `ReturnMainMenu`
  (`KismetSystemLibrary.Delay` 2.0)
  (`GameplayStatics.OpenLevel` "Level2_Testing"))

(event `RestartLevel`
  (`KismetSystemLibrary.Delay` 0.2)
  (bind _returnvalue (`GameplayStatics.GetCurrentLevelName` true))
  (`GameplayStatics.OpenLevel` (`KismetStringLibrary.Conv_StringToName` _returnvalue)))

(fn `CompleteLevel`
  (if (`|EnumEquality` (`self.CurrentState`) "NewEnumerator1")
    (set `self.CurrentState` "NewEnumerator2")
    (`KismetSystemLibrary.K2_ClearAndInvalidateTimerHandle` (`self.CountdownTimerHandle`))
    (`KismetSystemLibrary.PrintString` "Won")
    (`self.ReturnMainMenu`)))

(fn `CountdownTick`
  (if (`|EnumEquality` (`self.CurrentState`) "NewEnumerator1")
    (set `self.RemainingTime` (`KismetMathLibrary.FMax` (- (`self.RemainingTime`) 1.0)))
    (`KismetSystemLibrary.PrintString` (`KismetStringLibrary.Conv_DoubleToString` (`self.RemainingTime`)) true true (struct :`G` 0.66 :`B` 1.0 :`A` 1.0) 0.9)
    (if (<= (`self.RemainingTime`) 0.0)
      (`self.FailLevel`))))

(fn `FailLevel`
  (if (`|EnumEquality` (`self.CurrentState`) "NewEnumerator1")
    (set `self.CurrentState` "NewEnumerator3")
    (`KismetSystemLibrary.K2_ClearAndInvalidateTimerHandle` (`self.CountdownTimerHandle`))
    (`KismetSystemLibrary.PrintString` "Level Failed!")
    (`self.RestartLevel`)))

(fn `RegisterCollection`
  (returns (WasCollected :type Boolean))
  (if (and (`|EnumEquality` (`self.CurrentState`) "NewEnumerator1") (`|EnumInequality` (`self.ObjectiveMode`) "NewEnumerator0") (< (`self.CollectedItems`) (`self.RequiredItems`)))
    (set `self.CollectedItems` (+ (`self.CollectedItems`) 1))
    (set `self.FinishUnlocked` (>= (`self.CollectedItems`) (`self.RequiredItems`)))
    (`KismetSystemLibrary.PrintString` (`KismetStringLibrary.Conv_IntToString` (`self.CollectedItems`)) true true (struct :`G` 0.66 :`B` 1.0 :`A` 1.0) 3.0)
    (return true)
    (else
      (return false))))

(fn `StartLevel`
  (if (`|EnumEquality` (`self.CurrentState`) "NewEnumerator0")
    (set `self.CurrentState` "NewEnumerator1")
    (set `self.FinishUnlocked` (`|EnumEquality` (`self.ObjectiveMode`) "NewEnumerator0"))
    (`KismetSystemLibrary.PrintString` "Level Started")
    (if (`|EnumEquality` (`self.ObjectiveMode`) "NewEnumerator0")
      (set `self.RemainingTime` (`self.TimeLimit`))
      (bind _returnvalue (`KismetSystemLibrary.K2_SetTimer` null "CountdownTick" 1.0 true))
      (set `self.CountdownTimerHandle` _returnvalue))))

(fn `TryFinish`
  (if (`|EnumEquality` (`self.CurrentState`) "NewEnumerator1")
    (if (`self.FinishUnlocked`)
      (`self.CompleteLevel`)
      (else
        (`KismetSystemLibrary.PrintString` "Locked - Collect more items!")))))

(fn `UserConstructionScript`)