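; BP_Marble is a player-controlled physics marble that rolls, jumps and steers in the air relative to the camera.
; Each tick a downward sphere trace sets grounded state, applying full roll torque on ground or half torque plus an air force otherwise.
; Enhanced Input drives movement, look and a grounded velocity-change jump with a short cooldown.
; A charge value fills from BeginPlay but nothing spends it; the Boost input is empty.
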(event `self.ReceiveBeginPlay`
  (`EnhancedInputSubsystemInterface.AddMappingContext` (subsystem `EnhancedInputLocalPlayerSubsystem`) "/Game/Input/IMC_Default.IMC_Default" 0 (struct))
  (set `self.bIsCharging` true)
  (set `self.ChargeValue` 0.0))

(event `self.ReceiveTick`
  (params (DeltaSeconds :type "Float (single-precision)"))
  (bind _returnvalue (`self.K2_GetActorLocation`))
  (bind _rolltorque (`self.RollTorque`))
  (bind (_outhit _returnvalue_2) (`KismetSystemLibrary.SphereTraceSingle` _returnvalue (- _returnvalue (0.0 0.0 12.0)) 45.0 "TraceTypeQuery1"))
  (set `self.bIsGrounded` _returnvalue_2)
  (if (`self.bIsGrounded`)
    (`self.ApplyMarbleTorque` _rolltorque)
    (else
      (`self.ApplyMarbleTorque` (/ _rolltorque 2.0))
      (`self.ApplyAirForce`)))
  (if (and (`self.bIsCharging`) (< (`self.ChargeValue`) 1.0))
    (set `self.ChargeValue` (+ (`self.ChargeValue`) (* (`self.ChargeRate`) DeltaSeconds))))
  (set `self.ChargeValue` (`KismetMathLibrary.FClamp` (`self.ChargeValue`))))

(event `EnhancedInput|/Game/Input/Actions/IA_Move`
  (params (ActionValue :type "Vector2D Structure") (ElapsedSeconds :type "Float (double-precision)") (TriggeredSeconds :type "Float (double-precision)") (InputAction :type "InputAction Object Reference" :default "/Game/Input/Actions/IA_Move.IA_Move"))
  (:`Triggered`
    (set `self.MoveInput` (`KismetMathLibrary.Conv_Vector2DToVector` ActionValue)))
  (:`Canceled`
    (set `self.MoveInput` (0.0 0.0 0.0) :!label _label))
  (:`Completed`
    (goto _label)))

(event `EnhancedInput|/Game/Input/Actions/IA_Jump`
  (params (ActionValue :type Boolean) (ElapsedSeconds :type "Float (double-precision)") (TriggeredSeconds :type "Float (double-precision)") (InputAction :type "InputAction Object Reference" :default "/Game/Input/Actions/IA_Jump.IA_Jump"))
  (:`Triggered`
    (if (and (`self.bIsGrounded`) (`self.bCanJump`))
      (`PrimitiveComponent.AddImpulse` (`self.Sphere`) (`KismetMathLibrary.MakeVector` 0.0 0.0 (`self.JumpImpulse`)) "None" true)
      (set `self.bCanJump` false)
      (`KismetSystemLibrary.Delay` 0.2)
      (set `self.bCanJump` true))))

(event `EnhancedInput|/Game/BallGame/Input/IA_Boost`
  (params (ActionValue :type Boolean) (ElapsedSeconds :type "Float (double-precision)") (TriggeredSeconds :type "Float (double-precision)") (InputAction :type "InputAction Object Reference" :default "/Game/BallGame/Input/IA_Boost.IA_Boost")))

(event `EnhancedInput|/Game/Input/Actions/IA_Look`
  (params (ActionValue :type "Vector2D Structure") (ElapsedSeconds :type "Float (double-precision)") (TriggeredSeconds :type "Float (double-precision)") (InputAction :type "InputAction Object Reference" :default "/Game/Input/Actions/IA_Look.IA_Look"))
  (bind (_x _y) (`KismetMathLibrary.BreakVector2D` ActionValue))
  (:`Triggered`
    (`self.AddControllerYawInput` _x)
    (`self.AddControllerPitchInput` (* _y -1.0))))

(fn `ApplyAirForce`
  (locals (DirectionVector :type "Vector Structure"))
  (bind (_forward _right) (`self.GetCameraBasis`))
  (bind (_moveinput_x _moveinput_y) (`KismetMathLibrary.BreakVector` (`self.MoveInput`)))
  (bind _output_get (set `local.DirectionVector` (`KismetMathLibrary.Vector_Normal2D` (+ (* _moveinput_x _right) (* _moveinput_y _forward)))))
  (`PrimitiveComponent.AddForce` (`self.Sphere`) (* _output_get 200.0) "None" true))

(fn `ApplyMarbleTorque`
  (params (TorqueAmount :type "Float (double-precision)"))
  (locals (DirectionVector :type "Vector Structure") (TorqueAxis :type "Vector Structure") (TorqueVector :type "Vector Structure"))
  (bind (_forward _right) (`self.GetCameraBasis`))
  (bind (_moveinput_x _moveinput_y) (`KismetMathLibrary.BreakVector` (`self.MoveInput`)))
  (bind _output_get (set `local.DirectionVector` (`KismetMathLibrary.Vector_Normal2D` (+ (* _moveinput_x _right) (* _moveinput_y _forward)))))
  (bind _output_get_2 (set `local.TorqueAxis` (`KismetMathLibrary.Cross_VectorVector` (0.0 0.0 1.0) _output_get)))
  (bind _output_get_3 (set `local.TorqueVector` (* _output_get_2 TorqueAmount)))
  (`PrimitiveComponent.AddTorqueInRadians` (`self.Sphere`) _output_get_3 "None" true))

(fn `GetCameraBasis`
  (returns (Forward :type "Vector Structure") (Right :type "Vector Structure"))
  (bind _returnvalue (`PlayerCameraManager.GetCameraRotation` (`GameplayStatics.GetPlayerCameraManager` 0)))
  (bind (_returnvalue_x _returnvalue_y) (`KismetMathLibrary.BreakVector` (`KismetMathLibrary.GetForwardVector` _returnvalue)))
  (bind (_returnvalue_x_2 _returnvalue_y_2) (`KismetMathLibrary.BreakVector` (`KismetMathLibrary.GetRightVector` _returnvalue)))
  (return (`KismetMathLibrary.Vector_Normal2D` (`KismetMathLibrary.MakeVector` _returnvalue_x _returnvalue_y)) (`KismetMathLibrary.Vector_Normal2D` (`KismetMathLibrary.MakeVector` _returnvalue_x_2 _returnvalue_y_2))))

(fn `UserConstructionScript`)